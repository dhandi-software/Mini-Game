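; BP_Enemy is a stationary shooter enemy that turns to face the player and repeatedly fires BP_Projectile from a scene point on a delay loop.
; Its construction script snaps the gun mesh to the GunSocket.
; Hit clears the body mesh, spawns BP_DestructibleEnemy and a BP_Gun thrown toward the player with spin.
; A brief timer delays destruction so the lingering collider shatters the destructible mesh, working around APEX damage.
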(event Custom|Fire
  (bind _playerref (Variables|Default|GetPlayerRef))
  (bind _scene (Variables|Default|GetScene))
  (bind _returnvalue (Transformation|GetWorldLocation _scene))
  (bind _returnvalue_2 (Transformation|GetActorLocation _playerref))
  (bind _returnvalue_3 (Math|Rotator|FindLookatRotation _returnvalue _returnvalue_2))
  (if (not (Variables|Default|GetbIsDead))
    (Game|SpawnActorfromClass "/Game/Blueprints/BP_Projectile.BP_Projectile_C" (Math|Transform|MakeTransform _returnvalue (Math|Rotator|MakeRotator (.roll _returnvalue_3) 0.0 (.yaw _returnvalue_3)) "1.000000,1.000000,1.000000") "AlwaysSpawn" "OverrideRootScale" 0 0)
    (Utilities|FlowControl|Delay (Variables|Default|GetTimeBetweenShots))
    (CallFunction|Fire)))

(event EventBeginPlay
  (Variables|Default|SetPlayerRef (Game|Player|GetPlayerPawn 0))
  (Utilities|FlowControl|Delay (Variables|Default|GetTimeBetweenShots))
  (CallFunction|Fire))

(event EventTick
  (params (DeltaSeconds :type Float%20%28single-precision%29))
  (if (not (Variables|Default|GetbIsDead))
    (Transformation|SetActorRotation (Math|Rotator|FindLookatRotation (Transformation|GetActorLocation) (Transformation|GetActorLocation (Variables|Default|GetPlayerRef))))))

(fn ConstructionScript
  (Transformation|AttachComponentToComponent (Variables|Default|GetSkeletalMesh) (Variables|Character|GetMesh) "GunSocket" "SnapToTarget" "SnapToTarget" "SnapToTarget" true))

(fn Hit
  (if (not (Variables|Default|GetbIsDead))
    (Variables|Default|SetbIsDead true)
    (Components|SkinnedMesh|SetSkinnedAssetandUpdate (Variables|Character|GetMesh) 0 true)
    (Game|SpawnActorfromClass "/Game/Blueprints/BP_DestructibleEnemy.BP_DestructibleEnemy_C" (Transformation|GetWorldTransform (Variables|Character|GetMesh)) "AlwaysSpawn" "OverrideRootScale" 0 0)
    (bind _returnvalue (Game|SpawnActorfromClass "/Game/Blueprints/BP_Gun.BP_Gun_C" (Transformation|GetWorldTransform (Variables|Default|GetSkeletalMesh)) "AlwaysSpawn" "OverrideRootScale" 0 0))
    (Default|Thrown _returnvalue)
    ;[0 0 0] Tambahkan sejumlah kecil rotasi ke pistol berdasarkan penambahan gaya pada offset dari titik pivot objek.
    (Physics|AddImpulseatLocation (Variables|/Game/Blueprints/BP_Gun.BP_Gun_C|GetBox _returnvalue) "50.000000,50.000000,50.000000" (- (Transformation|GetWorldLocation (Variables|/Game/Blueprints/BP_Gun.BP_Gun_C|GetBox _returnvalue)) "0.000000,0.000000,2.000000") "None")
    ;[0 0 0] Melempar senjata ke arah pemain
    (Physics|AddImpulse (Variables|/Game/Blueprints/BP_Gun.BP_Gun_C|GetBox _returnvalue) (* (+ (Math|Vector|GetForwardVector (Transformation|GetWorldRotation (Variables|Collision|GetCapsuleComponent))) "0.000000, 0,0.200000") (Variables|Default|GetThrowVelocity)) "None" true)
    ;[0 0 0] Kita membutuhkan kelas musuh dan collidernya untuk tetap aktif selama sepersekian detik karena inilah yang sebenarnya menyebabkan destructibleEnemy mesh yang ditelurkan untuk dihancurkan. Menambahkan kerusakan pada penghancuran APEX yang lama tampaknya tidak berfungsi, jadi ini adalah cara mengakalinya.
    (Utilities|Time|SetTimerbyFunctionName 0 "DestroyEnemy" 0.001)))

(fn DestroyEnemy
  (Actor|DestroyActor))