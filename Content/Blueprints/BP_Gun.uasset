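; BP_Gun is the player's pistol, which can be fired, picked up and thrown.
; Fire plays a muzzle emitter and gun animation and spawns a BP_Projectile aimed along the player's first-person camera, gated by a delay-based cooldown.
; Collected and Thrown toggle physics and collision on the Box component.
; When the Box hits a BP_Enemy, it calls that enemy's Hit, so a thrown gun also works as a weapon.
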(event OnComponentHit(Box)
  (params (HitComponent :type Primitive%20Component%20Object%20Reference) (OtherActor :type Actor%20Object%20Reference) (OtherComp :type Primitive%20Component%20Object%20Reference) (NormalImpulse :type Vector :default "0, 0, 0") (Hit :type Hit%20Result%20Structure%20%28by%20ref%29))
  (bind _asbp_enemy (Utilities|Casting|CastToBP_Enemy OtherActor))
  (Default|Hit _asbp_enemy))

(event Custom|ResetFireCooldown
  (Utilities|FlowControl|Delay (Variables|Default|GetTimeBetweenShots))
  (Variables|Default|SetbCanFire true))

(event EventBeginPlay
  (bind _asbp_player (Utilities|Casting|CastToBP_Player (Game|Player|GetPlayerPawn 0)))
  (Variables|Default|SetPlayerRef _asbp_player))

(fn ConstructionScript)

(fn Fire
  (if (Variables|Default|GetbCanFire)
    (Variables|Default|SetbCanFire false)
    (Effects|SpawnEmitteratLocation "/Game/Assets2/Effects/P_PlayerExplosion.P_PlayerExplosion" (Transformation|GetWorldLocation (Variables|Default|GetScene)) (Transformation|GetActorRotation) "0.040000,0.040000,0.040000")
    (Game|SpawnActorfromClass "/Game/Blueprints/BP_Projectile.BP_Projectile_C" (Math|Transform|MakeTransform (Transformation|GetWorldLocation (Variables|Default|GetScene)) (Transformation|GetWorldRotation (Variables|/Game/Blueprints/BP_Player.BP_Player_C|GetFirstPersonCamera (Variables|Default|GetPlayerRef)))) "AdjustIfPossibleButDontSpawnIfColliding" "OverrideRootScale" 0 0) ; Spawn projectile
    (CallFunction|ResetFireCooldown)
    (Components|Animation|PlayAnimation (Variables|Default|GetFP_Gun) "/Game/Assets2/Meshes/Jericho_941_Anim.Jericho_941_Anim" false)))

(fn Collected
  (bind _box (Variables|Default|GetBox))
  (Class|PrimitiveComponent|SetAllPhysicsLinearVelocity (Variables|Default|GetBox) "0, 0, 0" false)
  (Physics|SetSimulatePhysics _box false)
  (Collision|SetCollisionEnabled _box "NoCollision"))

(fn Thrown
  (bind _box (Variables|Default|GetBox))
  (Physics|SetSimulatePhysics _box true)
  (Collision|SetCollisionEnabled _box "QueryAndPhysics"))