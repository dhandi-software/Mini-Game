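; Base component for a player rune, handling its activation and deactivation.
; On BeginPlay it binds to the player's activate and force-deactivate rune events.
; Activation toggles the component if its rune type is currently selected and disables it otherwise, which covers swapping runes.
; Enabling and disabling set an active flag and switch component tick on or off, while force-deactivation always disables.
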(event Custom|IsActiveComponent
  (CallFunction|CheckActiveStatus))

(event Custom|ForceRuneDeactivate
  (CallFunction|DisableRune))

(event EventBeginPlay
  (EventDispatchers|BindEventtoForceDeactivateRuneEvent (Variables|Default|GetPlayerRef) (delegate Custom|ForceRuneDeactivate))
  (EventDispatchers|AssignActivateRuneEvent (Variables|Default|GetPlayerRef) (delegate Custom|IsActiveComponent)))

(event EventTick
  (params (DeltaSeconds :type Float%20%28single-precision%29)))

(fn CheckActiveStatus
  (if (Utilities|Enum|Equal(Enum) (Variables|/Game/Blueprints/Game/BP_Player.BP_Player_C|GetCurrentlySelectedRune (Variables|Default|GetPlayerRef)) (Variables|Default|GetRuneType))
    (if (not (Variables|Default|GetbComponentActive))
      (CallFunction|EnableRune)
      (else
        (CallFunction|DisableRune)))
    (else
      ;[0 0 0] Call this to account for having swapped to another Rune to ensure rune  is disabled
      (CallFunction|DisableRune))))

(fn EnableRune
  (Components|Tick|SetComponentTickEnabled true)
  (Variables|Default|SetbComponentActive true))

(fn DisableRune
  (Components|Tick|SetComponentTickEnabled false)
  (Variables|Default|SetbComponentActive false))