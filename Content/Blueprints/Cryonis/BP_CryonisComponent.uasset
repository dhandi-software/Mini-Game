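; Cryonis rune component that lets the player raise ice pillars on surfaces of a custom collision channel.
; While active, Tick traces from the camera and spawns, moves or destroys a ghost preview at the impact point.
; The player's use-rune event spawns a cube at the ghost's transform unless the ghost reports it is blocked.
; At most three cubes exist at once, with the oldest destroyed to make room.
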(event Custom|SpawnCryoCube
  (CallFunction|SpawnCryonisPillar))

(event EventBeginPlay
  (|CallParentFunction)
  (EventDispatchers|BindEventtoUseActiveRuneEvent (Variables|Default|GetPlayerRef) (delegate Custom|SpawnCryoCube)))

(event EventDisableRune
  (|CallParentFunction)
  (Utilities|IsValid (Variables|Default|GetCryoGhost)
    (:Is%20Valid
      (Actor|DestroyActor (Variables|Default|GetCryoGhost)))
    (:Is%20Not%20Valid
      _))
  (Variables|Default|SetCryoGhost 0))

(event EventTick
  (params (DeltaSeconds :type Float%20%28single-precision%29))
  (if (Variables|Default|GetbComponentActive)
    (CallFunction|CheckPillarSpawnLocation)))

(event EventEnableRune
  (|CallParentFunction)
  (bind _returnvalue (Game|SpawnActorfromClass "/Game/Blueprints/Cryonis/BP_CryonisGhost.BP_CryonisGhost_C" (Math|Transform|MakeTransform "0, 0, 0" "0, 0, 0" "1,1,1") "Undefined" 0 0))
  (Variables|Default|SetCryoGhost _returnvalue))

(fn SpawnCryonisPillar
  (bind _cryoghost (Variables|Default|GetCryoGhost))
  (if (Variables|Default|GetbComponentActive)
    (Utilities|IsValid _cryoghost
      (:Is%20Valid
        (if (not (Variables|/Game/Blueprints/Cryonis/BP_CryonisGhost.BP_CryonisGhost_C|GetbSpawnBlocked _cryoghost))
          (if (== (Utilities|Array|Length (Variables|Default|GetActiveCryoCubes)) 3)
            (Actor|DestroyActor (Utilities|Array|Get(acopy) (Variables|Default|GetActiveCryoCubes)))
            (Utilities|Array|RemoveIndex (Variables|Default|GetActiveCryoCubes)))
          (bind _returnvalue (Game|SpawnActorfromClass "/Game/Blueprints/Cryonis/BP_CryonisCube.BP_CryonisCube_C" (Transformation|GetActorTransform (Variables|Default|GetCryoGhost)) "Undefined" 0 0))
          (Utilities|Array|AddUnique (Variables|Default|GetActiveCryoCubes) _returnvalue))))))

(fn CheckPillarSpawnLocation
  (bind _outhit (CallFunction|LinetracefromCamera))
  (bind (_bblockinghit _binitialoverlap _time _distance _location _impactpoint _normal _impactnormal _physmat _hitactor _hitcomponent) (Collision|BreakHitResult _outhit))
  (Utilities|IsValid _hitcomponent
    (:Is%20Valid
      (if (Utilities|Enum|Equal(Enum) (Collision|GetCollisionObjectType _hitcomponent) "ECC_GameTraceChannel1")
        (Utilities|IsValid (Variables|Default|GetCryoGhost)
          (:Is%20Valid
            _)
          (:Is%20Not%20Valid
            (bind _returnvalue (Game|SpawnActorfromClass "/Game/Blueprints/Cryonis/BP_CryonisGhost.BP_CryonisGhost_C" (Math|Transform|MakeTransform "0, 0, 0" (Transformation|GetWorldRotation _hitcomponent) "1,1,1") "Undefined" 0 0))
            (Variables|Default|SetCryoGhost _returnvalue)))
        (Transformation|SetActorLocation (Variables|Default|GetCryoGhost) _impactpoint false false)
        (else
          (Utilities|IsValid (Variables|Default|GetCryoGhost)
            (:Is%20Valid
              (Actor|DestroyActor (Variables|Default|GetCryoGhost))
              (Variables|Default|SetCryoGhost 0))))))
    (:Is%20Not%20Valid
      (Utilities|IsValid (Variables|Default|GetCryoGhost)
        (:Is%20Valid
          (Actor|DestroyActor (Variables|Default|GetCryoGhost))
          (Variables|Default|SetCryoGhost 0))))))