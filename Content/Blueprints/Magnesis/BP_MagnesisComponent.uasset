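; Magnesis rune component that lets the player grab, hold and push or pull metal BP_MagnesisActorBase objects.
; Enabling or disabling the rune swaps every magnesis actor's material and releases the physics handle.
; A camera line trace toggles grabbing through the player's PhysicsHandle, with a looping timer instead of Tick updating the hold target and beam particle.
; Push and pull slide the player's PhysicsObjectHold along its forward vector.
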(event Custom|PickupMagnesisObject
  (CallFunction|GrabMagnesisObject))

(event Custom|PushObject
  (CallFunction|PushPullObject true))

(event Custom|PullObject
  (CallFunction|PushPullObject false))

(event EventBeginPlay
  (|CallParentFunction)
  (EventDispatchers|BindEventtoUseActiveRuneEvent (Variables|Default|GetPlayerRef) (delegate Custom|PickupMagnesisObject))
  (EventDispatchers|BindEventtoPushMagEvent (Variables|Default|GetPlayerRef) (delegate Custom|PushObject))
  (EventDispatchers|AssignPullMagEvent (Variables|Default|GetPlayerRef) (delegate Custom|PullObject)))

(event EventTick
  (params (DeltaSeconds :type Float%20%28single-precision%29)))

(event EventEnableRune
  (|CallParentFunction)
  (CallFunction|HighlightAllMagnesisObjects true))

(event EventDisableRune
  (bind _beamparticle (Variables|Default|GetBeamParticle))
  (|CallParentFunction)
  (CallFunction|HighlightAllMagnesisObjects false)
  (Utilities|IsValid _beamparticle
    (:Is%20Valid
      (Components|DestroyComponent _beamparticle))))

(fn GetPlayerPhysicsHoldLocRot
  (return (Transformation|GetWorldLocation (CallFunction|GetPlayerPhysicsObjectHold)) (.yaw (Transformation|GetWorldRotation (CallFunction|GetPlayerPhysicsObjectHold)))))

(fn GetPlayerPhysicsHandle
  (return (Variables|/Game/Blueprints/Game/BP_Player.BP_Player_C|GetPhysicsHandle (Variables|Default|GetPlayerRef))))

(fn GetPlayerPhysicsObjectHold
  (return (Variables|/Game/Blueprints/Game/BP_Player.BP_Player_C|GetPhysicsObjectHold (Variables|Default|GetPlayerRef))))

(fn HighlightAllMagnesisObjects
  (params (IsActiveComponent :type Boolean))
  (bind _outactors (Actor|GetAllActorsOfClass "/Game/Blueprints/Magnesis/BP_MagnesisActorBase.BP_MagnesisActorBase_C"))
  (for _array_element _outactors
    (Rendering|Material|SetMaterial (Variables|/Game/Blueprints/Magnesis/BP_MagnesisActorBase.BP_MagnesisActorBase_C|GetStaticMesh _array_element) 0 (select IsActiveComponent "/Game/Assets/Materials/Magnesis/MI_MagGlowPink.MI_MagGlowPink" "/Game/Assets/Materials/Magnesis/MI_MagMetal.MI_MagMetal")))
  (Physics|Components|PhysicsHandle|ReleaseComponent (CallFunction|GetPlayerPhysicsHandle)))

(fn GrabMagnesisObject
  (bind (_returnvalue _returnvalue_yaw) (CallFunction|GetPlayerPhysicsHoldLocRot))
  (bind _outhit (CallFunction|LinetracefromCamera))
  (bind (_bblockinghit _binitialoverlap _time _distance _location _impactpoint _normal _impactnormal _physmat _hitactor _hitcomponent) (Collision|BreakHitResult _outhit))
  (if (Variables|Default|GetbComponentActive)
    (Utilities|IsValid (Variables|Default|GetMagnesisObject)
      (:Is%20Valid
        (Rendering|Material|SetMaterial (Variables|Default|GetMagnesisObject) 0 "/Game/Assets/Materials/Magnesis/MI_MagGlowPink.MI_MagGlowPink")
        (Utilities|Time|ClearTimerbyFunctionName 0 "UpdateHeldObject")
        (Physics|Components|PhysicsHandle|ReleaseComponent (CallFunction|GetPlayerPhysicsHandle))
        (Variables|Default|SetMagnesisObject 0)
        (Utilities|IsValid (Variables|Default|GetBeamParticle)
          (:Is%20Valid
            (Components|DestroyComponent (Variables|Default|GetBeamParticle)))))
      (:Is%20Not%20Valid
        (if _bblockinghit
          (Utilities|Casting|CastToBP_MagnesisActorBase _hitactor
            (:then
              (bind _output_get (Variables|Default|SetMagnesisObject _hitcomponent))
              (Rendering|Material|SetMaterial _output_get 0 "/Game/Assets/Materials/Magnesis/MI_MagGlowYellow.MI_MagGlowYellow")
              (Transformation|SetWorldLocation (CallFunction|GetPlayerPhysicsObjectHold) (Transformation|GetWorldLocation (Variables|Default|GetMagnesisObject)) false false)
              (Physics|Components|PhysicsHandle|GrabComponentatLocationwithRotation (CallFunction|GetPlayerPhysicsHandle) (Variables|Default|GetMagnesisObject) "None" _returnvalue (Math|Rotator|MakeRotator 0.0 0.0 _returnvalue_yaw))
              (bind _returnvalue_2 (Effects|SpawnEmitteratLocation "/Game/Assets/Effects/P_Beam.P_Beam" "0, 0, 0"))
              (Variables|Default|SetBeamParticle _returnvalue_2)
              ;[1 1 1] Loop Call to hold object in place with PhysicsHandle
              (Utilities|Time|SetTimerbyFunctionName 0 "UpdateHeldObject" 0.001 true))
            (:CastFailed
              (Variables|Default|SetMagnesisObject 0)))
          (else
            (Variables|Default|SetMagnesisObject 0)))))))

(fn UpdateHeldObject
  (bind (_returnvalue _returnvalue_yaw) (CallFunction|GetPlayerPhysicsHoldLocRot))
  (bind _beamparticle (Variables|Default|GetBeamParticle))
  (bind _beamparticle_2 (Variables|Default|GetBeamParticle))
  (bind _beamparticle_3 (Variables|Default|GetBeamParticle))
  (Class|PhysicsHandleComponent|SetTargetLocationandRotation (CallFunction|GetPlayerPhysicsHandle) _returnvalue (Math|Rotator|MakeRotator 0.0 0.0 _returnvalue_yaw))
  (Utilities|IsValid (Variables|Default|GetBeamParticle)
    (:Is%20Valid
      ;[1 1 1] Update each emitter in the beam particle to follow the object
      (Class|ParticleSystemComponent|SetBeamSourcePoint _beamparticle_2 0 (Transformation|GetActorLocation (Variables|Default|GetPlayerRef)))
      (Class|ParticleSystemComponent|SetBeamTargetPoint _beamparticle_2 0 (Transformation|GetWorldLocation (Variables|Default|GetMagnesisObject)))
      (Class|ParticleSystemComponent|SetBeamSourcePoint _beamparticle_3 1 (Transformation|GetActorLocation (Variables|Default|GetPlayerRef)))
      (Class|ParticleSystemComponent|SetBeamTargetPoint _beamparticle_3 1 (Transformation|GetWorldLocation (Variables|Default|GetMagnesisObject)))
      (Class|ParticleSystemComponent|SetBeamSourcePoint _beamparticle 2 (Transformation|GetActorLocation (Variables|Default|GetPlayerRef)))
      (Class|ParticleSystemComponent|SetBeamTargetPoint _beamparticle 2 (Transformation|GetWorldLocation (Variables|Default|GetMagnesisObject))))))

(fn PushPullObject
  (params (IsPushing :type Boolean))
  (bind _physicsobjecthold (CallFunction|GetPlayerPhysicsObjectHold))
  (bind _returnvalue (Math|Vector|GetForwardVector _physicsobjecthold))
  (Transformation|SetWorldLocation (CallFunction|GetPlayerPhysicsObjectHold) (+ (Transformation|GetWorldLocation _physicsobjecthold) (* (select IsPushing _returnvalue (Math|Vector|NegateVector _returnvalue)) (LocalVariables|GetMoveForce))) false false))